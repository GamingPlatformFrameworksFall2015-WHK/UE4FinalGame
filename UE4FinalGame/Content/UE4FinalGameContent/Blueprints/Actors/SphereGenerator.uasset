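; SphereGenerator is an actor that spawns teleport beacons in a sphere-shaped grid around its location at BeginPlay.
; Nested loops over latitude and longitude line counts call PlaceBeacon, which converts each index pair to a point using spherical-coordinate math expressions.
; Each beacon spawns unrotated at that offset, uniformly scaled by the sphere radius relative to the latitude line count.
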(event EventActorBeginOverlap
  (params (OtherActor :type Actor%20Object%20Reference)))

(event EventTick
  (params (DeltaSeconds :type Float%20%28single-precision%29)))

(event EventBeginPlay
  (bind _longlines (Variables|Default|GetlongLines))
  (bind _radius (Variables|Default|Getradius))
  (bind _latlines (Variables|Default|GetlatLines))
  (for _index (range 0 _latlines)
    (for _index_2 (range 0 _longlines)
      (bind (_x _y _z) (CallFunction|PlaceBeacon _index _latlines _index_2 _longlines _radius))
      (Game|SpawnActorfromClass (Variables|Default|GetteleportBeaconClass) (Math|Transform|MakeTransform (+ (Math|Vector|MakeVector _x _y _z) (Transformation|GetActorLocation)) "0, 0, 0" (Math|Conversions|ToVector(Float) (|(sphereRadius*(1/(lines*100))) (Math|Conversions|ToFloat(Integer) _latlines) (Math|Conversions|ToFloat(Integer) _radius)))) "Undefined" 0 0))))

(fn ConstructionScript)

(fn PlaceBeacon
  (params (m :type Integer) (lat :type Integer) (n :type Integer) (long :type Integer) (radius :type Integer))
  (bind _returnvalue (Math|Trig|GetPI))
  (bind _returnvalue_2 (Math|Conversions|ToFloat(Integer) m))
  (bind _returnvalue_3 (Math|Conversions|ToFloat(Integer) lat))
  (bind _returnvalue_4 (Math|Conversions|ToFloat(Integer) n))
  (bind _returnvalue_5 (Math|Conversions|ToFloat(Integer) long))
  (return (* radius (|((sin((Pi*(m/lat))))*(cos(((2*Pi)*(n/long))))) _returnvalue _returnvalue_2 _returnvalue_3 _returnvalue_4 _returnvalue_5)) (* radius (Math|Trig|Sin(Radians) _returnvalue _returnvalue_2 _returnvalue_3 _returnvalue_4 _returnvalue_5)) (* radius (Math|Trig|Cos(Degrees) _returnvalue _returnvalue_2 _returnvalue_3))))