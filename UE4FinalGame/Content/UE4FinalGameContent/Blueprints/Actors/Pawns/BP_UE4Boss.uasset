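; Boss pawn that turns to face the player and shoots projectiles from its attack point.
; Tick interpolates the mesh toward the player at RotationSpeed, calls FireWeapons, and draws a debug trace along the muzzle's forward vector.
; FireWeapons relies on a Delay ignoring per-tick retriggers to space projectile spawns by FireInterval, with a laser sound.
; FireMissiles spawns a homing projectile with an explosion sound, but nothing in this graph calls it.
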(event `Update Rotation`
  ;[1 1 1] Boss Rotation
  (`SceneComponent.K2_SetWorldRotation` (`self.BossStaticMesh`) (`KismetMathLibrary.RInterpTo` (`SceneComponent.K2_GetComponentRotation` (`self.BossStaticMesh`)) (`KismetMathLibrary.MakeRotator` (.roll (`KismetMathLibrary.FindLookAtRotation` (`SceneComponent.K2_GetComponentLocation` (`self.BossStaticMesh`)) (`self.K2_GetActorLocation` (`GameplayStatics.GetPlayerCharacter` 0)))) (.pitch (`KismetMathLibrary.FindLookAtRotation` (`SceneComponent.K2_GetComponentLocation` (`self.BossStaticMesh`)) (`self.K2_GetActorLocation` (`GameplayStatics.GetPlayerCharacter` 0)))) (.yaw (`KismetMathLibrary.FindLookAtRotation` (`SceneComponent.K2_GetComponentLocation` (`self.BossStaticMesh`)) (`self.K2_GetActorLocation` (`GameplayStatics.GetPlayerCharacter` 0))))) (`self.DeltaTime`) (`self.RotationSpeed`)) false false))

(event `self.ReceiveBeginPlay`)

(event `self.ReceiveActorBeginOverlap`
  (params (OtherActor :type "Actor Object Reference")))

(event `Fire Weapons`
  ;[1 1 1] Firing AI
  (`KismetSystemLibrary.Delay` (`self.FireInterval`))
  (`|SpawnActorFromClass` "/Game/FirstPersonCPP/Blueprints/FirstPersonProjectile.FirstPersonProjectile_C" (`SceneComponent.GetSocketTransform` (`self.BulletSpawnPoint`) "BossAttackPoint" "RTS_World") "Undefined" "OverrideRootScale")
  (`GameplayStatics.PlaySoundAtLocation` "/Game/UE4FinalGameContent/laser_fire.laser_fire" (`self.K2_GetActorLocation`)))

(event `self.ReceiveTick`
  (params (DeltaSeconds :type "Float (single-precision)"))
  (bind _bulletspawnpoint (`self.BulletSpawnPoint`))
  (bind _returnvalue (`SceneComponent.K2_GetComponentLocation` _bulletspawnpoint))
  (set `self.DeltaTime` DeltaSeconds)
  (`self.Update Rotation`)
  (`self.Fire Weapons`)
  (`KismetSystemLibrary.LineTraceSingle` :`Start` _returnvalue :`End` (+ _returnvalue (* (`KismetMathLibrary.GetForwardVector` (`SceneComponent.K2_GetComponentRotation` _bulletspawnpoint)) 100000)) :`TraceChannel` "TraceTypeQuery1" :`DrawDebugType` "ForDuration"))

(event `Fire Missiles`
  (`|SpawnActorFromClass` "/Game/UE4FinalGameContent/Blueprints/Actors/FirstPersonHomingProjectile.FirstPersonHomingProjectile_C" (`SceneComponent.GetSocketTransform` (`self.BulletSpawnPoint`) "BossAttackPoint" "RTS_World") "Undefined" "OverrideRootScale")
  (`GameplayStatics.PlaySoundAtLocation` "/Game/StarterContent/Audio/Explosion01.Explosion01" (`self.K2_GetActorLocation`)))

(fn `UserConstructionScript`)